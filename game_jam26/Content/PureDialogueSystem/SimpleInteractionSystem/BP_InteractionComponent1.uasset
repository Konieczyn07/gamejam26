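; Actor component that lets its owning Character detect and interact with BPI_Interactable actors.
; Capsule overlap events maintain a list of interactables in range, which shows or hides a lazily created WBP_InteractionWidget with text supplied by the target.
; On BeginPlay it adds the IMC_InteractionSystem mapping context, and IA_Interact sends InteractMessage to the target.
; Despite its name, GetClosestInteractionWidget returns the first actor in the list, with no distance check.
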(event `self.ReceiveBeginPlay`
  ;[1 0.53 0.6303] Assign Custom event on the owner characters capsule
  (bind _ascharacter (cast `Character` (`self.GetOwner`)))
  (set `self.CharacterRef` _ascharacter)
  (bind _capsulecomponent (`Character.CapsuleComponent` _ascharacter))
  (add `PrimitiveComponent.OnComponentBeginOverlap` _capsulecomponent (`|CreateDelegate` :!event `OnComponentBeginOverlap_Event`))
  (add `PrimitiveComponent.OnComponentEndOverlap` _capsulecomponent (`|CreateDelegate` :!event `CustomEvent`))
  (bind _asplayer_controller (cast `PlayerController` (`Pawn.GetController` (`self.CharacterRef`))))
  (`EnhancedInputSubsystemInterface.AddMappingContext` (pcsubsystem `EnhancedInputLocalPlayerSubsystem` _asplayer_controller) "/Game/PureDialogueSystem/SimpleInteractionSystem/Input/IMC_InteractionSystem.IMC_InteractionSystem" 0 (struct)))

(event `OnComponentBeginOverlap_Event`
  (params (OverlappedComponent :type "PrimitiveComponent Object Reference") (OtherActor :type "Actor Object Reference") (OtherComp :type "PrimitiveComponent Object Reference") (OtherBodyIndex :type Integer) (bFromSweep :type Boolean) (SweepResult :type "HitResult Structure (by ref)"))
  ;[0.5512 1 0.8369] When The Owner character is overlaped with any of the Interactables. Show Interaction Widget
  (if (`KismetSystemLibrary.DoesImplementInterface` OtherActor "/Game/PureDialogueSystem/SimpleInteractionSystem/BPI_Interactable.BPI_Interactable_C")
    (`KismetArrayLibrary.Array_Add` (`self.InteractionsInRange`) OtherActor)
    (`self.RenderInteractionWidget`)))

(event `CustomEvent`
  (params (OverlappedComponent :type "PrimitiveComponent Object Reference") (OtherActor :type "Actor Object Reference") (OtherComp :type "PrimitiveComponent Object Reference") (OtherBodyIndex :type Integer))
  ;[0.9624 0.5758 1] When Owner Character moves away from any interactable. Hide The Interaction Widget
  (if (`KismetSystemLibrary.DoesImplementInterface` OtherActor "/Game/PureDialogueSystem/SimpleInteractionSystem/BPI_Interactable.BPI_Interactable_C")
    (`KismetArrayLibrary.Array_RemoveItem` (`self.InteractionsInRange`) OtherActor)
    (`self.RenderInteractionWidget`)))

(event `EnhancedInput|/Game/PureDialogueSystem/SimpleInteractionSystem/Input/IA_Interact`
  (params (ActionValue :type Boolean) (ElapsedSeconds :type "Float (double-precision)") (TriggeredSeconds :type "Float (double-precision)") (InputAction :type "InputAction Object Reference" :default "/Game/PureDialogueSystem/SimpleInteractionSystem/Input/IA_Interact.IA_Interact"))
  ;[0.6937 1 0.447] When INteract Input is pressed. check if the character is close to any of the interactable actors. If any interactable are close Interact
  (:`Started`
    (if (> (`KismetArrayLibrary.Array_Length` (`self.InteractionsInRange`)) 0)
      (message `/Game/PureDialogueSystem/SimpleInteractionSystem/BPI_Interactable.Interact` (`self.GetClosestInteractionWidget`) (`self.GetOwner`)))))

(fn `GetClosestInteractionWidget`
  (returns (Actor :type "Actor Object Reference"))
  (`/Engine/EditorBlueprintResources/StandardMacros.IsValid` (`|GetArrayItem` (`self.InteractionsInRange`))
    (:`Is Valid`
      (return (`|GetArrayItem` (`self.InteractionsInRange`))))))

(fn `RenderInteractionWidget`
  (if (> (`KismetArrayLibrary.Array_Length` (`self.InteractionsInRange`)) 0)
    (`|ExecutionSequence`
      (:`then_0`
        ;[0.901 0.6008 1] If Interaction is not valid create the widget first.
        (`/Engine/EditorBlueprintResources/StandardMacros.IsValid` (`self.InteractionWidgetRef`)
          (:`Is Not Valid`
            (bind _asplayer_controller (cast `PlayerController` (`Pawn.GetController` (`self.CharacterRef`))))
            (bind _returnvalue (`|CreateWidget` "/Game/PureDialogueSystem/SimpleInteractionSystem/WBP_InteractionWidget.WBP_InteractionWidget_C" _asplayer_controller))
            (bind _output_get (set `self.InteractionWidgetRef` _returnvalue))
            (`UserWidget.AddToViewport` _output_get -1))))
      (:`then_1`
        ;[0.8217 1 0.9801] Show Interaction Widget. And update its text from the interactable actor. Eg Pickup, Open/Close Door.
        (`/Game/PureDialogueSystem/SimpleInteractionSystem/WBP_InteractionWidget.ShowInteractionWidget` (`self.InteractionWidgetRef`))
        (bind _text (message `/Game/PureDialogueSystem/SimpleInteractionSystem/BPI_Interactable.GetInteractionText` (`self.GetClosestInteractionWidget`)))
        (`/Game/PureDialogueSystem/SimpleInteractionSystem/WBP_InteractionWidget.UpdateInteractionText` (`self.InteractionWidgetRef`) _text)))
    (else
      ;[1 0.2188 0.4305] Hide Interaction WIdget
      (`/Engine/EditorBlueprintResources/StandardMacros.IsValid` (`self.InteractionWidgetRef`)
        (:`Is Valid`
          (`/Game/PureDialogueSystem/SimpleInteractionSystem/WBP_InteractionWidget.HideInteractionWidget` (`self.InteractionWidgetRef`)))))))