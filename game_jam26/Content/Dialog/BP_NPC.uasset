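; BP_NPC is a talkable NPC that shows a widget when the player character overlaps its Trigger and hides it when the player leaves.
; Non-player overlaps apply the opposite visibility in each case.
; The Talk event is empty.
; Disconnected nodes hold an unfinished dialogue sequence that switches to UI input, steps through Dialog lines and displays them in a WBP_Dialog widget, so it never runs.
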(event `/Game/Dialog/BPI_Dialog.Talk`
  ; shit dialogue ig
)

(event `self.Trigger.OnComponentBeginOverlap`
  (params (OverlappedComponent :type "PrimitiveComponent Object Reference") (OtherActor :type "Actor Object Reference") (OtherComp :type "PrimitiveComponent Object Reference") (OtherBodyIndex :type Integer) (bFromSweep :type Boolean) (SweepResult :type "HitResult Structure (by ref)"))
  (bind _widget (`self.Widget`))
  (cast `/Game/ThirdPerson/Blueprints/BP_ThirdPersonCharacter` OtherActor
    (:`then`
      (`SceneComponent.SetVisibility` _widget true false))
    (:`CastFailed`
      (`SceneComponent.SetVisibility` _widget false false))))

(event `self.Trigger.OnComponentEndOverlap`
  (params (OverlappedComponent :type "PrimitiveComponent Object Reference") (OtherActor :type "Actor Object Reference") (OtherComp :type "PrimitiveComponent Object Reference") (OtherBodyIndex :type Integer))
  (bind _widget (`self.Widget`))
  (cast `/Game/ThirdPerson/Blueprints/BP_ThirdPersonCharacter` OtherActor
    (:`then`
      (`SceneComponent.SetVisibility` _widget false false))
    (:`CastFailed`
      (`SceneComponent.SetVisibility` _widget true false))))

(fn `UserConstructionScript`)