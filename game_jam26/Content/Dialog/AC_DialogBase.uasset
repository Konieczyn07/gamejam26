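; AC_DialogBase is a base dialogue component that opens a conversation widget and tracks the options chosen at each step.
; The empty Convo function is a hook for child scripts, replayed from the start whenever ProgressConvo runs.
; AddConvo returns stored choices for answered steps or shows the current line in W_Convo, and UpdateSelectedOption records a choice and replays.
; Helpers roll back progress or switch tree index, clearing progress.
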(fn `AddConvo`
  (params (Speaker :type Text) (Convo :type Text) (`Options Text` :type "Array of Text"))
  (returns (State :type "/Game/Dialog/Dialog_State Enum") (`Option Index` :type Integer))
  (bind (_value _returnvalue) (`BlueprintMapLibrary.Map_Find` (`self.ConvoProgress`) (`self.ConvoIndex`)))
  (`/Engine/EditorBlueprintResources/StandardMacros.IncrementInt` (`self.ConvoIndex`)
    (:`  `
      (if _returnvalue
        (return "NewEnumerator0" _value)
        (else
          (`/Game/UI/HUD/W_Convo.UpdateConvoText` (`self.ConvoWidget`) (`self.ConvoIndex`) (`local.Speaker`) (`local.Convo`) (`local.Options Text`))
          (return "NewEnumerator1" 0))))))

(fn `ClearConvoProgress`
  (`BlueprintMapLibrary.Map_Clear` (`self.ConvoProgress`)))

(fn `CloseConvo`
  (`Widget.RemoveFromParent` (`self.ConvoWidget`)))

(fn `Convo`)

(fn `OpenConvo`
  (bind _returnvalue (`|CreateWidget` "/Game/UI/HUD/W_Convo.W_Convo_C" null self))
  (bind _output_get (set `self.ConvoWidget` _returnvalue))
  (`UserWidget.AddToViewport` _output_get 0)
  (`self.ProgressConvo`))

(fn `ProgressConvo`
  (set `self.ConvoIndex` -1)
  (`self.Convo`))

(fn `RemoveConvoProgress`
  (params (ProgressSteps :type Integer))
  (for _index (range (+ ProgressSteps 1))
    (`BlueprintMapLibrary.Map_Remove` (`self.ConvoProgress`) (- (`self.ConvoIndex`) _index))))

(fn `SetConvoTreeIndex`
  (params (ConvoTreeIndex :type Integer))
  (set `self.ConvoTreeIndex` ConvoTreeIndex)
  (`self.ClearConvoProgress`))

(fn `UpdateSelectedOption`
  (params (Progress :type "Integer (by ref)") (OptionIndex :type "Integer (by ref)"))
  (`BlueprintMapLibrary.Map_Add` (`self.ConvoProgress`) Progress OptionIndex)
  (`self.ProgressConvo`))